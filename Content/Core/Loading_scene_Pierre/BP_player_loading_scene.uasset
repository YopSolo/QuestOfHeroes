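; Player character for the loading scene that moves sideways, hops upward and drops rain while airborne.
; Jump launches it upward without a ground check, gated by a DoOnce that resets after a short delay, so hops can repeat mid-air.
; While falling, a random Delay on Tick throttles spawning of small BP_rain_drop actors below it with a random Y offset.
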(event EventBeginPlay)

(event EventTick
  (params (DeltaSeconds :type Float%20%28single-precision%29))
  (if (AI|Components|NavMovement|IsFalling (Variables|Character|GetCharacterMovement))
    (Utilities|FlowControl|Delay (Math|Random|RandomFloatinRange 0.1 0.4))
    (Game|SpawnActorfromClass "/Game/Core/Loading_scene_Pierre/BP_rain_drop.BP_rain_drop_C" (Math|Transform|MakeTransform (- (Transformation|GetActorLocation) (Math|Vector|MakeVector 0.0 (Math|Random|RandomFloatinRange 2e+01 -2e+01) 5e+01)) "0, 0, 0" "0.200000,0.200000,0.200000") "AlwaysSpawn" 0 0)))

(event Input|ActionEvents|InputActionJump
  (params (Key :type Key%20Structure :default "None"))
  (:Pressed
    (Utilities|FlowControl|DoOnce false :!label _label
      (:Completed
        (Character|LaunchCharacter "0, 0,150.000000" false true)
        (Utilities|FlowControl|Delay 0.3)
        (goto _label Reset)))))

(event Input|AxisEvents|InputAxisMoveRight/Left
  (params (AxisValue :type Float%20%28single-precision%29))
  (Pawn|Input|AddMovementInput (Transformation|GetActorRightVector) AxisValue false))

(fn ConstructionScript)